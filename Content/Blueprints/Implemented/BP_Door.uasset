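; BP_Door is a double door that swings open or closed each time its Interaction event fires.
; A FlipFlop alternates between playing and reversing the MovementDoor timeline, whose play rate is set from SpeedOpening so that value acts as a duration.
; The timeline track, scaled by RotationAngle, yaws the left and right door meshes in opposite directions.
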(event EventInteraction
  (Components|Timeline|SetPlayRate (Variables|Default|GetMovementDoor) (/ 1.0 (Variables|Default|GetSpeedOpening)))
  (Utilities|FlowControl|FlipFlop
    (:A
      (bind _newtrack_0 (Timeline|MovementDoor Play)
        (:Update
          (Transformation|SetRelativeRotation (Variables|Default|GetSM_DoorL) (Math|Rotator|MakeRotator 0.0 0.0 (* (* _newtrack_0 (Variables|Default|GetRotationAngle)) -1.0)) false false)
          (Transformation|SetRelativeRotation (Variables|Default|GetSM_DoorR) (Math|Rotator|MakeRotator 0.0 0.0 (* _newtrack_0 (Variables|Default|GetRotationAngle))) false false))))
    (:B
      (Timeline|MovementDoor Reverse))))

(fn ConstructionScript)